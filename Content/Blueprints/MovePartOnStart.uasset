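; Actor Blueprint for a part that moves out to a random spot on start, as in an explode effect.
; BeginPlay sets the target by adding an offset to the actor's location, fixed slightly along negative world X and random in Y and Z.
; Tick moves the actor toward that target at constant Speed with VInterpToConstant, without sweeping for collision.
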(event `self.ReceiveBeginPlay`
  ; Set a random location for the part to move towards on start (explode)
  (bind _output_get (set `self.CurrentPos` (`self.K2_GetActorLocation`)))
  (bind _output_get_2 (set `self.RandomOffset` (`KismetMathLibrary.MakeVector` -10.0 (`KismetMathLibrary.RandomFloatInRange` -100.0 100.0) (`KismetMathLibrary.RandomFloatInRange` -100.0 100.0))))
  (set `self.TargetPos` (+ _output_get _output_get_2)))

(event `self.ReceiveTick`
  (params (DeltaSeconds :type "Float (single-precision)"))
  ; Move part to target location
  (set `self.FrameTime` DeltaSeconds)
  (bind _output_get (set `self.CurrentPos` (`KismetMathLibrary.VInterpTo_Constant` (`self.CurrentPos`) (`self.TargetPos`) (`self.FrameTime`) (`self.Speed`))))
  (`self.K2_SetActorLocation` _output_get))

(fn `UserConstructionScript`)